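; Game manager Blueprint that runs a button-sequence puzzle and ends it with a win or lose screen.
; ButtonPressed checks each ID against CorrectOrder at CurrentIndex, advancing on a match, winning when the sequence completes and losing on any mismatch.
; Both outcomes call RestartLevel, which resets the index, disables player input and movement, and shows the result widget with cursor and UI-only input, without reloading the level.
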(event `RestartLevel`
  (params (hasWon :type Boolean))
  (bind _returnvalue (`GameplayStatics.GetPlayerCharacter` 0))
  (bind _returnvalue_2 (`GameplayStatics.GetPlayerController` 0))
  (set `self.CurrentIndex` 0)
  (`self.DisableInput` _returnvalue _returnvalue_2)
  (`NavMovementInterface.StopActiveMovement` (`Character.CharacterMovement` _returnvalue))
  (if hasWon
    (bind _returnvalue_3 (`|CreateWidget` "/Game/Blueprints/WBP_WinScreen.WBP_WinScreen_C" _returnvalue_2))
    (`UserWidget.AddToViewport` _returnvalue_3 0)
    (set `PlayerController.bShowMouseCursor` true _returnvalue_2)
    (`WidgetBlueprintLibrary.SetInputMode_UIOnlyEx` _returnvalue_2 _returnvalue_3)
    (else
      (bind _returnvalue_4 (`|CreateWidget` "/Game/Blueprints/WBP_LoseScreen.WBP_LoseScreen_C" _returnvalue_2))
      (`UserWidget.AddToViewport` _returnvalue_4 0)
      (set `PlayerController.bShowMouseCursor` true _returnvalue_2)
      (`WidgetBlueprintLibrary.SetInputMode_UIOnlyEx` _returnvalue_2 _returnvalue_4))))

(event `ButtonPressed`
  (params (ButtonID :type Integer))
  (if (== ButtonID (`|GetArrayItem` (`self.CorrectOrder`) (`self.CurrentIndex`)))
    (bind _result (`/Engine/EditorBlueprintResources/StandardMacros.IncrementInt` (`self.CurrentIndex`))
      (:`  `
        (if (== (`KismetArrayLibrary.Array_Length` (`self.CorrectOrder`)) _result)
          (`self.RestartLevel` true))))
    (else
      (`self.RestartLevel` false))))

(fn `UserConstructionScript`)